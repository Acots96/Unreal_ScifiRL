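; BP_ScoreVFX is a score pickup actor with a Capsule trigger and a Niagara trail component.
; On BeginPlay it binds the capsule overlap; an actor carrying TargetActorTag adds Score through GM_Game, then the pickup destroys itself.
; A sine/cosine circular offset for the trail exists but is disconnected, so Tick does nothing.
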(event `self.ReceiveBeginPlay`
  (add `PrimitiveComponent.OnComponentBeginOverlap` (`self.Capsule`) (delegate `OnComponentBeginOverlap_Event`)))

(event `OnComponentBeginOverlap_Event`
  (params (OverlappedComponent :type "PrimitiveComponent Object Reference") (OtherActor :type "Actor Object Reference") (OtherComp :type "PrimitiveComponent Object Reference") (OtherBodyIndex :type Integer) (bFromSweep :type Boolean) (SweepResult :type "HitResult Structure (by ref)"))
  (if (`self.ActorHasTag` OtherActor (`self.TargetActorTag`))
    (bind _asgm_game (cast `/Game/_Main/GM_Game` (`GameplayStatics.GetGameMode`)))
    (`/Game/_Main/GM_Game.AddScore` _asgm_game (`self.Score`))
    (`self.K2_DestroyActor`)))

(event `self.ReceiveTick`
  (params (DeltaSeconds :type "Float (single-precision)")))

(fn `UserConstructionScript`)