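; Missile projectile that launches along a randomized upward arc, then flies on toward DesiredTarget.
; On BeginPlay it builds four control points, which Tick follows using a recursive De Casteljau Bézier evaluation while measuring its speed.
; After the curve it eases to Speed and steers toward the target with a downward bias, turning less sharply as speed rises.
; Once at or below the target's height, it holds its forward heading.
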(event `self.ReceiveBeginPlay`
  (`parent.ReceiveBeginPlay`)
  (`self.InitSplinePoints`))

(event `self.ReceiveTick`
  (params (DeltaSeconds :type "Float (single-precision)"))
  (bind _currentalpha (`self.CurrentAlpha`))
  (if (<= _currentalpha 1.0)
    (bind _output_get (set `self.CurrentAlpha` (+ _currentalpha (* DeltaSeconds (`self.AlphaMultiplier`)))))
    (set `self.LastLoc` (`self.K2_GetActorLocation`))
    (bind (_position _direction) (`self.ComputeSplinePosition` _output_get (`self.SplinePoints`)))
    (`self.K2_SetActorLocationAndRotation` _position (`KismetMathLibrary.MakeRotFromX` _direction))
    (set `self.CurrentSpeed` (/ (`KismetMathLibrary.Vector_Distance` (`self.K2_GetActorLocation`) (`self.LastLoc`)) DeltaSeconds))
    (else
      (set `self.CurrentSpeed` (`KismetMathLibrary.Lerp` (`self.CurrentSpeed`) (`self.Speed`) 0.1))
      (`self.K2_AddActorWorldOffset` (- (* DeltaSeconds (`self.CurrentSpeed`) (`self.GetActorForwardVector`)) (0.0 0.0 0.0)))
      (`self.K2_SetActorRotation` (`KismetMathLibrary.RLerp` (`self.K2_GetActorRotation`) (`self.ComputeTargetRotation`) (`KismetMathLibrary.FClamp` (- 0.75 (/ (`self.CurrentSpeed`) (`self.Speed`))) 0.02 0.3) true)))))

(fn `ComputeSplinePosition`
  (params (Alpha :type "Float (double-precision)") (Points :type "Array of Vector Structure"))
  (returns (Position :type "Vector Structure") (Direction :type "Vector Structure"))
  (locals (Local_Points :type "Array of Vector Structure") (Local_Alpha :type "Float (double-precision)"))
  (bind _returnvalue (`KismetArrayLibrary.Array_Length` Points))
  (bind _output (`|GetArrayItem` Points))
  (bind _output_2 (`|GetArrayItem` Points 1))
  (set `local.Local_Alpha` Alpha)
  (if (== _returnvalue 2)
    (return (`KismetMathLibrary.VLerp` _output _output_2 (`local.Local_Alpha`)) (`KismetMathLibrary.Normal` (- _output_2 _output)))
    (else
      (for _index (range (+ (- _returnvalue 2) 1))
        (`KismetArrayLibrary.Array_Add` (`local.Local_Points`) (`KismetMathLibrary.VLerp` (`|GetArrayItem` Points _index) (`|GetArrayItem` Points (+ _index 1)) (`local.Local_Alpha`))))
      (bind (_position _direction) (`self.ComputeSplinePosition` (`local.Local_Alpha`) (`local.Local_Points`)))
      (return _position _direction))))

(fn `ComputeTargetRotation`
  (returns (TargetRot :type "Rotator Structure"))
  (bind (_returnvalue_x _returnvalue_y _returnvalue_z) (`KismetMathLibrary.BreakVector` (`self.K2_GetActorLocation`)))
  (bind (_returnvalue_x_2 _returnvalue_y_2 _returnvalue_z_2) (`KismetMathLibrary.BreakVector` (`self.K2_GetActorLocation` (`self.DesiredTarget`))))
  (bind (_returnvalue_x_3 _returnvalue_y_3) (`KismetMathLibrary.BreakVector` (- (`self.K2_GetActorLocation` (`self.DesiredTarget`)) (`self.K2_GetActorLocation`))))
  (if (<= _returnvalue_z _returnvalue_z_2)
    (return (`KismetMathLibrary.MakeRotFromX` (`self.GetActorForwardVector`)))
    (else
      (return (`KismetMathLibrary.MakeRotFromX` (`KismetMathLibrary.Normal` (`KismetMathLibrary.MakeVector` _returnvalue_x_3 _returnvalue_y_3 -100.0)))))))

(fn `InitSplinePoints`
  (bind _returnvalue (`self.K2_GetActorLocation`))
  (bind _output_get (set `self.SplinePoints` (`|MakeArray` _returnvalue (+ _returnvalue (* (`self.GetActorForwardVector`) 10.0)) (+ _returnvalue (* (`KismetMathLibrary.Vector_Up`) (`KismetMathLibrary.RandomFloatInRange` 250.0 350.0)) (* (`self.GetActorForwardVector`) 150.0) (* (`self.GetActorRightVector`) 150.0 (- (* (`KismetMathLibrary.RandomFloat`) 2.0) 1.0))))))
  (bind _output (`|GetArrayItem` _output_get 2))
  (`KismetArrayLibrary.Array_Add` _output_get (+ (* (`KismetMathLibrary.Normal` (- (`self.K2_GetActorLocation` (`self.DesiredTarget`)) _output)) 200.0) _output)))

(fn `UserConstructionScript`
  (`parent.UserConstructionScript`))