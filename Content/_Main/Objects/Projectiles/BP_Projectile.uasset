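; Projectile actor that flies straight along its spawn forward vector at a set speed, moved each Tick without sweep, and expires after its lifetime.
; Overlaps on the Shot component ignore the owner, damage tag-matched targets through their HealthComponent, and destroy the projectile on those targets or WorldStatic objects.
; On impact it spawns a Niagara VFX actor, tinted with a brightened copy of the Shot material's Color parameter.
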(event `self.ReceiveBeginPlay`
  (set `self.Direction` (`self.GetActorForwardVector`))
  (`self.SetLifeSpan` (`self.LifeTime`))
  (add `PrimitiveComponent.OnComponentBeginOverlap` (`self.Shot`) (delegate `OnOverlap`)))

(event `OnOverlap`
  (params (OverlappedComponent :type "PrimitiveComponent Object Reference") (OtherActor :type "Actor Object Reference") (OtherComp :type "PrimitiveComponent Object Reference") (OtherBodyIndex :type Integer) (bFromSweep :type Boolean) (SweepResult :type "HitResult Structure (by ref)"))
  (bind _returnvalue (`self.GetComponentByClass` OtherActor "/Game/_Main/Components/HealthComponent.HealthComponent_C"))
  (if (!= OtherActor (`self.GetOwner`))
    (if (and (`/Game/_Main/Utils.AnyTag` (`self.TargetTags`) (`Actor.Tags` OtherActor)) (`KismetSystemLibrary.IsValid` _returnvalue))
      (`/Game/_Main/Components/HealthComponent.TakeDamage` _returnvalue (`self.Damage`) (`self.GetOwner`))
      (`self.SpawnImpactVFX` :!label _label)
      (`self.K2_DestroyActor`)
      (elif (`|EnumEquality` (`PrimitiveComponent.GetCollisionObjectType` OtherComp) "ECC_WorldStatic")
        (goto _label)))))

(event `self.ReceiveTick`
  (params (DeltaSeconds :type "Float (single-precision)"))
  (`self.K2_AddActorWorldOffset` (* DeltaSeconds (`self.Speed`) (`self.Direction`))))

(fn `SpawnImpactVFX`
  (bind _returnvalue (`|SpawnActorFromClass` (`self.BP_ImpactVFX`) (`KismetMathLibrary.MakeTransform` (`self.K2_GetActorLocation`)) "Undefined" "MultiplyWithRoot" null null))
  (bind _returnvalue_2 (`PrimitiveComponent.CreateDynamicMaterialInstance` (`self.Shot`) 0 null "None"))
  (bind _returnvalue_3 (`MaterialInstanceDynamic.K2_GetVectorParameterValue` _returnvalue_2 "Color"))
  (`NiagaraComponent.SetVariableLinearColor` (`/Game/_Main/Objects/VFX/BP_ImpactVFX.Niagara` _returnvalue) "User.Particle Color" (* _returnvalue_3 (struct :`R` 2.0 :`G` 2.0 :`B` 2.0 :`A` 1.0))))

(fn `UserConstructionScript`)