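; BP_CameraLab is a camera actor that continuously turns to face the player's BP_Character.
; On BeginPlay it caches the GM_Game game mode, then finds and stores the first BP_Character as its target, only if that cast succeeds.
; Each Tick it rotates the whole actor along the normalized direction from its Camera component to the target's center, with no smoothing or validity check.
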(event `self.ReceiveBeginPlay`
  (bind _asgm_game (cast `/Game/_Main/GM_Game` (`GameplayStatics.GetGameMode`)))
  (set `self.GM_Game` _asgm_game)
  (bind _returnvalue (`GameplayStatics.GetActorOfClass` "/Game/_Main/Characters/Main/BP_Character.BP_Character_C"))
  (set `self.Target` _returnvalue))

(event `self.ReceiveTick`
  (params (DeltaSeconds :type "Float (single-precision)"))
  (`self.K2_SetActorRotation` (`KismetMathLibrary.MakeRotFromX` (`KismetMathLibrary.Normal` (- (`/Game/_Main/Characters/Main/BP_Character.GetCenterLocation` (`self.Target`)) (`SceneComponent.K2_GetComponentLocation` (`self.Camera`)))))))

(fn `UserConstructionScript`)