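; Interactable monitor station that opens the character menu HUD through GM_Game when the player triggers its interact component.
; Capsule overlap registers that component on BP_Character, shows or clears the interact prompt, and flips the animation direction.
; Tick advances a clamped interpolation that swings both side screens through a float curve.
; Four cube meshes are hidden once opening nears completion and shown again as it reverses.
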(event `OnInteract`
  (`/Game/_Main/GM_Game.ShowCharacterMenuHUD` (`self.GM_Game`)))

(event `OnBeginEnd`
  (params (OverlappedComponent :type "PrimitiveComponent Object Reference") (OtherActor :type "Actor Object Reference") (OtherComp :type "PrimitiveComponent Object Reference") (OtherBodyIndex :type Integer))
  (if (`self.ActorHasTag` OtherActor "Player")
    (bind _asbp_character (cast `/Game/_Main/Characters/Main/BP_Character` OtherActor))
    (set `/Game/_Main/Characters/Main/BP_Character.CurrentInteractComp` null _asbp_character)
    (set `self.CharacterNear` null)
    (`SceneComponent.SetHiddenInGame` (`self.CanInteract_Widget`) true false)
    (`/Game/_Main/GM_Game.CleanMessageHUD` (`self.GM_Game`))
    (set `self.TargetInterpSign` -1.0)))

(event `OnBeginOverlap`
  (params (OverlappedComponent :type "PrimitiveComponent Object Reference") (OtherActor :type "Actor Object Reference") (OtherComp :type "PrimitiveComponent Object Reference") (OtherBodyIndex :type Integer) (bFromSweep :type Boolean) (SweepResult :type "HitResult Structure (by ref)"))
  (if (`self.ActorHasTag` OtherActor "Player")
    (bind _asbp_character (cast `/Game/_Main/Characters/Main/BP_Character` OtherActor))
    (set `/Game/_Main/Characters/Main/BP_Character.CurrentInteractComp` (`self.InteractComponent`) _asbp_character)
    (set `self.CharacterNear` _asbp_character)
    (`/Game/_Main/GM_Game.ShowMessageHUD` (`self.GM_Game`) "Press E to interact" 0.0)
    (set `self.TargetInterpSign` 1.0)))

(event `self.ReceiveBeginPlay`
  (bind _capsule (`self.Capsule`))
  (add `PrimitiveComponent.OnComponentBeginOverlap` _capsule (delegate `OnBeginOverlap`))
  (add `PrimitiveComponent.OnComponentEndOverlap` _capsule (delegate `OnBeginEnd`))
  (bind _asgm_game (cast `/Game/_Main/GM_Game` (`GameplayStatics.GetGameMode`)))
  (set `self.GM_Game` _asgm_game)
  (add `/Game/_Main/Components/InteractComponent.OnInteract` (`self.InteractComponent`) (delegate `OnInteract`)))

(event `self.ReceiveTick`
  (params (DeltaSeconds :type "Float (single-precision)"))
  (`self.RotateScreens` DeltaSeconds))

(fn `RotateScreens`
  (params (DeltaTime :type "Float (double-precision)"))
  (set `self.CurrentInterp` (`KismetMathLibrary.FClamp` (+ (* DeltaTime (`self.TargetInterpSign`) 0.75) (`self.CurrentInterp`))))
  (`|ExecutionSequence`
    (:`then_0`
      (if (and (>= (`self.CurrentInterp`) 0.8) (> (`self.TargetInterpSign`) 0.0))
        (`self.TurnScreensOnOff` true)
        (elif (and (< (`self.CurrentInterp`) 0.8) (< (`self.TargetInterpSign`) 0.0))
          (`self.TurnScreensOnOff` false))))
    (:`then_1`
      (`SceneComponent.K2_SetRelativeRotation` (`self.ScreenRight`) (`KismetMathLibrary.RLerp` (`KismetMathLibrary.MakeRotator` 0.0 0.0 120.0) (`KismetMathLibrary.MakeRotator` 0.0) (`CurveFloat.GetFloatValue` (`self.SideScreenCurve`) (`self.CurrentInterp`)) true) false false)
      (`SceneComponent.K2_SetRelativeRotation` (`self.ScreenLeft`) (`KismetMathLibrary.RLerp` (`KismetMathLibrary.MakeRotator` 0.0 0.0 -120.0) (`KismetMathLibrary.MakeRotator` 0.0) (`CurveFloat.GetFloatValue` (`self.SideScreenCurve`) (`self.CurrentInterp`)) true) false false))))

(fn `TurnScreensOnOff`
  (params (SetOFF :type Boolean))
  (`SceneComponent.SetHiddenInGame` (`self.Cube`) SetOFF false)
  (`SceneComponent.SetHiddenInGame` (`self.Cube1`) SetOFF false)
  (`SceneComponent.SetHiddenInGame` (`self.Cube2`) SetOFF false)
  (`SceneComponent.SetHiddenInGame` (`self.Cube3`) SetOFF false))

(fn `UserConstructionScript`)