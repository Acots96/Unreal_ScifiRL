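; Rifle weapon that spawns projectiles and triggers a laser muzzle effect, limited by fire delay and heat.
; TryShoot fires only when the delay has elapsed, heat is below 75% and the Shooter is nearly level, then adds heat.
; Tick counts down the delay and cools heat after a pause; reaching 75% triples that pause and halves cooling while above it.
; Aim and target setters only store values.
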(event `self.ReceiveBeginPlay`)

(event `self.ReceiveTick`
  (params (DeltaSeconds :type "Float (single-precision)"))
  (`|ExecutionSequence`
    (:`then_0`
      (`self.ComputeShootDelay` DeltaSeconds))
    (:`then_1`
      (`self.ComputeHeat` DeltaSeconds))))

(fn `ComputeHeat`
  (params (DeltaTime :type "Float (double-precision)"))
  (if (> (`self.StartHeatDecrDelayDelta`) 0.0)
    (set `self.StartHeatDecrDelayDelta` (- (`self.StartHeatDecrDelayDelta`) DeltaTime))
    (else
      (set `self.CurrentHeat` (`KismetMathLibrary.FMax` (- (`self.CurrentHeat`) (* DeltaTime (`self.HeatDecrPerSecond`) (`KismetMathLibrary.SelectFloat` 0.5 1.0 (>= (`self.GetHeatFraction`) 0.75)))))))))

(fn `ComputeShootDelay`
  (params (DeltaTime :type "Float (double-precision)"))
  (if (> (`self.FireDelayDelta`) 0.0)
    (set `self.FireDelayDelta` (- (`self.FireDelayDelta`) DeltaTime))))

(fn `GetHeatFraction`
  (returns (Fraction :type "Float (double-precision)"))
  (return (/ (`self.CurrentHeat`) (`self.MaxHeat`))))

(fn `SetAim`
  (params (IsAiming :type Boolean))
  (set `self.IsAiming` IsAiming))

(fn `SetTargetLocation`
  (params (TargetLocXY :type "Vector Structure"))
  (set `self.TargetLocXY` TargetLocXY))

(fn `TryShoot`
  (bind _shooter (`self.Shooter`))
  (bind (_returnvalue_location _returnvalue_rotation) (`KismetMathLibrary.BreakTransform` (`SceneComponent.K2_GetComponentToWorld` _shooter)))
  (bind (_returnvalue_roll _returnvalue_pitch) (`KismetMathLibrary.BreakRotator` (`SceneComponent.K2_GetComponentRotation` _shooter)))
  (if (and (<= (`self.FireDelayDelta`) 0.0) (< (`self.CurrentHeat`) (* (`self.MaxHeat`) 0.75)))
    (if (< (`KismetMathLibrary.Abs` _returnvalue_pitch) 5.0)
      (`|SpawnActorFromClass` (`self.BP_Projectile`) (`KismetMathLibrary.MakeTransform` _returnvalue_location _returnvalue_rotation) "Undefined" "OverrideRootScale" (`self.GetOwner`) (`self.TargetTags`) 10.0 null)
      (`ActorComponent.Activate` (`self.Niagara_LaserMuzzle`) true)
      (set `self.FireDelayDelta` (`self.FireDelay`))
      (set `self.CurrentHeat` (`KismetMathLibrary.FClamp` (+ (`self.CurrentHeat`) (`self.HeatPerShot`)) 0.0 (`self.MaxHeat`)))
      (set `self.StartHeatDecrDelayDelta` (* (`self.StartHeatDecrDelay`) (`KismetMathLibrary.SelectFloat` 3.0 1.0 (>= (`self.GetHeatFraction`) 0.75)))))))

(fn `UserConstructionScript`)