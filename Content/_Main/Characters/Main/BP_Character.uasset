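; Player character with mouse aiming that switches between a slow-walking lab hub and an arena, returning to the lab on death.
; InitArena/InitLab swap input contexts and spawn or destroy the equipped weapon; arena entry also applies the HP skill upgrade.
; Enhanced Input drives camera-relative movement, jumping, interaction, aim/shoot states and a montage-timed, curve-scaled dodge roll.
; Aiming projects the cursor onto the character's height plane, driving body rotation, turn-in-place flags and weapon yaw.
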(event Custom|OnMontageEnd
  (params (Montage :type Anim%20Montage%20Object%20Reference) (bInterrupted :type Boolean))
  (Variables|Default|SetIsDodging false)
  (CallFunction|SetRunSpeed))

(event Custom|Damaged
  (params (Damage :type Float%20%28double-precision%29) (Attacker :type Actor%20Object%20Reference))
  (Default|UpdateHUDHP (Variables|Default|GetGM_Game) (Default|GetFraction (Variables|Default|GetHealthComponent))))

(event Custom|Died
  (params (Damage :type Float%20%28double-precision%29) (Attacker :type Actor%20Object%20Reference))
  (Variables|Default|SetIsDead true)
  (Input|DisableInput (Variables|Default|GetPlayerCtrl))
  (Utilities|FlowControl|Delay 2.0)
  (CallFunction|InitLab)
  (Default|BacktoLab (Variables|Default|GetGM_Game))
  (Input|EnableInput (Variables|Default|GetPlayerCtrl)))

(event Input|EnhancedActionEvents|EnhancedInputActionIA_Move
  (params (ActionValue :type Vector%202D%20Structure) (ElapsedSeconds :type Float%20%28double-precision%29) (TriggeredSeconds :type Float%20%28double-precision%29) (InputAction :type Input%20Action%20Object%20Reference :default "/Game/_Main/Input/IA_Move.IA_Move"))
  (:Triggered
    (if (not (or (Variables|Default|GetIsDodging) (Variables|Default|GetIsInteracting)))
      (CallFunction|TickMovement (.x ActionValue) (.y ActionValue))
      (Variables|Default|SetInputXY (Math|Vector|MakeVector (.y ActionValue) (.x ActionValue) 0.0))))
  (:Canceled
    (Variables|Default|SetInputXY (Math|Vector|MakeVector (.y ActionValue) (.x ActionValue) 0.0) :!label _label))
  (:Completed
    (goto _label)))

(event Input|EnhancedActionEvents|EnhancedInputActionIA_Dodge
  (params (ActionValue :type Boolean) (ElapsedSeconds :type Float%20%28double-precision%29) (TriggeredSeconds :type Float%20%28double-precision%29) (InputAction :type Input%20Action%20Object%20Reference :default "/Game/_Main/Input/IA_Dodge.IA_Dodge"))
  (bind _mesh (Variables|Character|GetMesh))
  (bind _returnvalue (Components|SkeletalMesh|GetAnimInstance _mesh))
  (:Started
    (if (CallFunction|CanDoActions false)
      (Utilities|FlowControl|Sequence
        (:then_0
          (Variables|Default|SetIsDodging true)
          (CallFunction|ComputeTargetRollDir)
          (CallFunction|SetRollSpeed))
        (:then_1
          (EventDispatchers|BindEventtoOnMontageBlendingOut _returnvalue (delegate Custom|OnMontageEnd))
          (bind _returnvalue_2 (Animation|Montage|MontagePlay _returnvalue "/Game/_Main/Characters/Animations/RollMontage.RollMontage" 1.0 "MontageLength" 0.0 true))
          (Variables|Default|SetRollMontageDuration _returnvalue_2)
          (Variables|Default|SetCurrentDeltaTime 0.0))))))

(event Input|EnhancedActionEvents|EnhancedInputActionIA_Aim
  (params (ActionValue :type Boolean) (ElapsedSeconds :type Float%20%28double-precision%29) (TriggeredSeconds :type Float%20%28double-precision%29) (InputAction :type Input%20Action%20Object%20Reference :default "/Game/_Main/Input/IA_Aim.IA_Aim"))
  (:Triggered
    (if (CallFunction|CanDoActions false) :!label _label
      (CallFunction|SetAimat true)
      (CallFunction|SetWalkSpeed)))
  (:Started
    (goto _label))
  (:Canceled
    (if (CallFunction|CanDoActions false) :!label _label_2
      (CallFunction|SetAimat false)
      (CallFunction|SetRunSpeed)))
  (:Completed
    (goto _label_2)))

(event Input|EnhancedActionEvents|EnhancedInputActionIA_Shoot
  (params (ActionValue :type Boolean) (ElapsedSeconds :type Float%20%28double-precision%29) (TriggeredSeconds :type Float%20%28double-precision%29) (InputAction :type Input%20Action%20Object%20Reference :default "/Game/_Main/Input/IA_Shoot.IA_Shoot"))
  (:Triggered
    (if (not (or (Variables|Default|GetIsDodging) (Variables|Default|GetIsInteracting)))
      (bind _output_get (Variables|Default|SetIsShooting true))
      (CallFunction|SetAimat _output_get)
      (CallFunction|SetWalkSpeed)))
  (:Canceled
    (bind _output_get_2 (Variables|Default|SetIsShooting false :!label _label))
    (CallFunction|SetAimat _output_get_2)
    (CallFunction|SetRunSpeed))
  (:Completed
    (goto _label)))

(event Input|EnhancedActionEvents|EnhancedInputActionIA_Jump
  (params (ActionValue :type Boolean) (ElapsedSeconds :type Float%20%28double-precision%29) (TriggeredSeconds :type Float%20%28double-precision%29) (InputAction :type Input%20Action%20Object%20Reference :default "/Game/_Main/Input/IA_Jump.IA_Jump"))
  (:Started
    (if (not (or (AI|Components|NavMovement|IsFalling (Variables|Character|GetCharacterMovement)) (Variables|Default|GetIsInteracting)))
      (Character|Jump))))

(event Input|EnhancedActionEvents|EnhancedInputActionIA_Interact
  (params (ActionValue :type Boolean) (ElapsedSeconds :type Float%20%28double-precision%29) (TriggeredSeconds :type Float%20%28double-precision%29) (InputAction :type Input%20Action%20Object%20Reference :default "/Game/_Main/Input/IA_Interact.IA_Interact"))
  (bind _currentinteractcomp (Variables|Default|GetCurrentInteractComp))
  (:Started
    (if (Variables|Default|GetCanInteract)
      (Utilities|IsValid _currentinteractcomp
        (:Is%20Valid
          (Variables|Default|SetIsInteracting true)
          (Variables|Default|SetCanInteract false)
          (Default|Interact _currentinteractcomp))))))

(event EventBeginPlay
  (Utilities|FlowControl|Sequence
    (:then_0
      (bind _asplayer_controller (Utilities|Casting|CastToPlayerController (Pawn|GetController)))
      (bind _output_get (Variables|Default|SetPlayerCtrl _asplayer_controller))
      (Input|AddMappingContext (PlayerController|LocalPlayerSubsystems|GetEnhancedInputLocalPlayerSubsystem _output_get) "/Game/_Main/Input/IMC_Lab.IMC_Lab" 0 "(bIgnoreAllPressedKeysUntilRelease=True,bForceImmediately=False,bNotifyUserSettings=False)")
      (Variables|/Script/Engine.PlayerController|SetbShowMouseCursor _output_get true)
      (CallFunction|SetWalkSpeed))
    (:then_1
      (bind _asgm_game (Utilities|Casting|CastToGM_Game (Game|GetGameMode)))
      (Variables|Default|SetGM_Game _asgm_game)
      (EventDispatchers|BindEventtoOnDamaged (Variables|Default|GetHealthComponent) (delegate Custom|Damaged))
      (EventDispatchers|BindEventtoOnDied (Variables|Default|GetHealthComponent) (delegate Custom|Died)))))

(event EventTick
  (params (DeltaSeconds :type Float%20%28single-precision%29))
  (if (not (Variables|Default|GetIsInLab))
    (CallFunction|TickArena DeltaSeconds)))

(event Input|KeyboardEvents|DebugKeyQ
  (params (Key :type Key%20Structure :default "None") (ActionValue :type Input%20Action%20Value%20Structure))
  (:Released
    (Default|DeleteGameSlot (Variables|Default|GetGM_Game))
    (Game|QuitGame 0 "Quit" false)))

(event Input|KeyboardEvents|DebugKeyEscape
  (params (Key :type Key%20Structure :default "None") (ActionValue :type Input%20Action%20Value%20Structure))
  (:Released
    (Default|CloseCharacterMenuHUD (Variables|Default|GetGM_Game))))

(fn ConstructionScript)

(fn ComputeTargetRollDir
  (bind _inputxy (Variables|Default|GetInputXY))
  (if (Math|Vector|VectorIsNearlyZero _inputxy 0.01)
    (Variables|Default|SetTargetRollDir (Math|Rotator|MakeRotator 0.0 0.0 (.yaw (Math|Rotator|MakeRotfromX (Transformation|GetActorForwardVector)))))
    (else
      (Variables|Default|SetTargetRollDir (Math|Rotator|MakeRotator 0.0 0.0 (.yaw (Math|Rotator|MakeRotfromX (Math|Transform|TransformDirection (Transformation|GetWorldTransform (Variables|/Script/Engine.Actor|GetRootComponent (Variables|Default|GetCurrentCam))) _inputxy))))))))

(fn TickLookat
  (bind _returnvalue (Transformation|GetActorLocation))
  (Utilities|FlowControl|Sequence
    (:then_0
      (CallFunction|ComputeMouseLineTrace)
      (CallFunction|ComputeDeltaYaw)
      (CallFunction|ComputeAimingTurn90)
      (CallFunction|ApplyRotation))
    (:then_1
      (bind _output_get (Variables|Default|SetLocalVelocityLookAtXY (Math|Transform|InverseTransformDirection (Transformation|GetActorTransform) (Transformation|GetVelocity))))
      (Rendering|Debug|DrawDebugLine _returnvalue (+ _returnvalue (* _output_get 2e+02)) "(R=1.000000,G=0.036994,B=0.000000,A=1.000000)" 0.0 0.0)
      (if (not (Math|Vector|VectorIsNearlyZero (Transformation|GetVelocity)))
        (Transformation|SetActorRotation (Math|Rotator|Lerp(Rotator) (Transformation|GetActorRotation) (Math|Rotator|MakeRotator 0.0 0.0 (.yaw (Math|Rotator|FindLookatRotation (Transformation|GetActorLocation) (Variables|Default|GetTargetLookXY)))) 0.1 true))
        (Variables|/Script/Engine.CharacterMovementComponent|SetbOrientRotationToMovement (Variables|Character|GetCharacterMovement) false)))
    (:then_2
      (CallFunction|AdjustAimWeapon))))

(fn TickMovement
  (params (X :type Float%20%28single-precision%29) (Y :type Float%20%28single-precision%29))
  (bind _currentcam (Variables|Default|GetCurrentCam))
  (bind _rootcomponent (Variables|/Script/Engine.Actor|GetRootComponent _currentcam))
  (bind _returnvalue (Transformation|GetWorldRotation _rootcomponent))
  (bind _returnvalue_2 (Math|Vector|GetForwardVector _returnvalue))
  (bind _returnvalue_3 (Math|Vector|GetRightVector _returnvalue))
  (Pawn|Input|AddMovementInput (Math|Vector|Normalize (Math|Vector|MakeVector (.x _returnvalue_2) (.y _returnvalue_2) 0.0)) Y false)
  (Pawn|Input|AddMovementInput (Math|Vector|Normalize (Math|Vector|MakeVector (.x _returnvalue_3) (.y _returnvalue_3) 0.0)) X false))

(fn TickRoll
  (params (DeltaTime :type Float%20%28double-precision%29))
  (Transformation|SetActorRotation (Math|Rotator|Lerp(Rotator) (Transformation|GetActorRotation) (Variables|Default|GetTargetRollDir) 0.3 true))
  (bind _output_get (Variables|Default|SetCurrentDeltaTime (+ (Variables|Default|GetCurrentDeltaTime) DeltaTime)))
  (Pawn|Input|AddMovementInput (Math|Vector|GetForwardVector (Variables|Default|GetTargetRollDir)) (Math|Curves|GetFloatValue (Variables|Default|GetRollSpeedCurve) (/ _output_get (Variables|Default|GetRollMontageDuration))) false)
  (CallFunction|SetRollSpeed))

(fn TickShooting
  (params (DeltaTime :type Float%20%28double-precision%29))
  (if (<= (Variables|Default|GetCurrentDeltaDelayShotsTime) 0.0)
    (if (Variables|Default|GetIsShooting)
      (Variables|Default|SetIsAiming true)
      (Variables|Default|SetCurrentDeltaDelayShotsTime (Variables|Default|GetDelayBetweenShots)))
    (else
      (Variables|Default|SetCurrentDeltaDelayShotsTime (- (Variables|Default|GetCurrentDeltaDelayShotsTime) DeltaTime)))))

(fn SetWalkSpeed
  (bind _charactermovement (Variables|Character|GetCharacterMovement))
  (bind _charactermovement_2 (Variables|Character|GetCharacterMovement))
  (if (Variables|Default|GetIsInLab)
    (Variables|/Script/Engine.CharacterMovementComponent|SetMaxWalkSpeed _charactermovement 2e+02)
    (Variables|/Script/Engine.CharacterMovementComponent|SetMaxAcceleration _charactermovement 512.0)
    (Variables|/Script/Engine.CharacterMovementComponent|SetBrakingDecelerationWalking _charactermovement 16.0)
    (else
      (Variables|/Script/Engine.CharacterMovementComponent|SetMaxWalkSpeed _charactermovement_2 (Variables|Default|GetWalkSpeed))
      (Variables|/Script/Engine.CharacterMovementComponent|SetMaxAcceleration _charactermovement_2 512.0)
      (Variables|/Script/Engine.CharacterMovementComponent|SetBrakingDecelerationWalking _charactermovement_2 16.0))))

(fn SetRunSpeed
  (bind _charactermovement (Variables|Character|GetCharacterMovement))
  (Variables|/Script/Engine.CharacterMovementComponent|SetMaxWalkSpeed _charactermovement (Variables|Default|GetRunSpeed))
  (Variables|/Script/Engine.CharacterMovementComponent|SetMaxAcceleration _charactermovement 2048.0)
  (Variables|/Script/Engine.CharacterMovementComponent|SetBrakingDecelerationWalking _charactermovement 1024.0))

(fn SetRollSpeed
  (bind _charactermovement (Variables|Character|GetCharacterMovement))
  (Variables|/Script/Engine.CharacterMovementComponent|SetMaxWalkSpeed _charactermovement (Variables|Default|GetRollSpeed))
  (Variables|/Script/Engine.CharacterMovementComponent|SetMaxAcceleration _charactermovement 4096.0)
  (Variables|/Script/Engine.CharacterMovementComponent|SetBrakingDecelerationWalking _charactermovement 1024.0))

(fn SetAimat
  (params (IsAiming :type Boolean))
  (bind _output_get (Variables|Default|SetIsAiming (or IsAiming (Variables|Default|GetIsShooting))))
  (Variables|/Script/Engine.CharacterMovementComponent|SetbOrientRotationToMovement (Variables|Character|GetCharacterMovement) (not _output_get))
  (Default|SetAim (Variables|Default|GetCurrentWeapon) _output_get))

(fn ComputeDeltaYaw
  (bind _returnvalue (Transformation|GetActorLocation))
  (bind _returnvalue_2 (Transformation|GetActorForwardVector))
  (bind _targetlookxy (Variables|Default|GetTargetLookXY))
  (bind _returnvalue_3 (- _targetlookxy _returnvalue))
  (bind _returnvalue_4 (Math|Vector|Normalize (Math|Vector|MakeVector (.x _returnvalue_3) (.y _returnvalue_3) 0.0)))
  (bind _returnvalue_5 (Math|Vector|DotProduct _returnvalue_2 _returnvalue_4))
  (bind _returnvalue_6 (Class|KismetMathLibrary|DegAcos _returnvalue_5))
  (Variables|Default|SetAimDeltaYaw (Math|Float|SelectFloat (* _returnvalue_6 -1.0) _returnvalue_6 (< (Math|Vector|DotProduct (Transformation|GetActorRightVector) _returnvalue_4) 0.0))))

(fn ComputeAimingTurn90
  (if (Math|Vector|VectorIsNearlyZero (Transformation|GetVelocity))
    (if (> (Math|Float|Absolute(Float) (Variables|Default|GetAimDeltaYaw)) 6e+01)
      (if (> (Variables|Default|GetAimDeltaYaw) 0.0)
        (Variables|Default|SetIsTurningRight true)
        (else
          (Variables|Default|SetIsTurningLeft true)))
      (elif (< (Math|Float|Absolute(Float) (Variables|Default|GetAimDeltaYaw)) 5.0)
        (Variables|Default|SetIsTurningRight false :!label _label)
        (Variables|Default|SetIsTurningLeft false)))
    (else
      (goto _label))))

(fn SpawnWeapon
  (params (ItemData :type Item%20Data%20Asset%20Object%20Reference))
  (bind _mesh (Variables|Character|GetMesh))
  (bind _returnvalue (Game|SpawnActorfromClass (Variables|/Game/_Main/Data/Items/ItemDataAsset.ItemDataAsset_C|GetItemBP ItemData) (Transformation|GetSocketTransform _mesh "Hand_R_Socket" "RTS_World") "Undefined" "MultiplyWithRoot" 0 0))
  (bind _asbp_weapon (Utilities|Casting|CastToBP_Weapon _returnvalue))
  (Variables|Default|SetCurrentWeapon _asbp_weapon)
  (Transformation|AttachComponentToComponent _returnvalue _mesh "Hand_RSocket" "SnapToTarget" "SnapToTarget" "SnapToTarget" true))

(fn GetHandLIK
  (bind _currentweapon (Variables|Default|GetCurrentWeapon))
  (bind _mesh (Variables|Character|GetMesh))
  (bind _staticmesh (Variables|/Game/_Main/Objects/Weapons/BP_Weapon.BP_Weapon_C|GetStaticMesh _currentweapon))
  (bind _returnvalue (Transformation|GetSocketTransform _staticmesh "Hand_L_Socket" "RTS_World"))
  (bind (_outposition _outrotation) (Class|SkinnedMeshComponent|TransformtoBoneSpace _mesh "Hand_R" (.location _returnvalue) (.rotation _returnvalue)))
  (if (Transformation|DoesSocketExist _staticmesh "Hand_L_Socket")
    (return (Math|Transform|MakeTransform _outposition _outrotation))))

(fn GetShootDelay
  (return (Variables|/Game/_Main/Objects/Weapons/BP_Rifle.BP_Rifle_C|GetFireDelay (Variables|Default|GetCurrentWeapon))))

(fn TryShoot
  (Default|TryShoot (Variables|Default|GetCurrentWeapon)))

(fn ComputeMouseLineTrace
  (bind _playerctrl (Variables|Default|GetPlayerCtrl))
  (bind (_worldlocation _worlddirection) (Game|Player|ConvertMouseLocationToWorldSpace _playerctrl))
  (bind (_outhit _returnvalue) (Collision|LineTraceByChannel _worldlocation (+ _worldlocation (* _worlddirection 2e+04)) "TraceTypeQuery2" false 0 "ForOneFrame"))
  (if _returnvalue
    (bind _targetpoint (CallFunction|GetTargetLocAccordingtoZ _worldlocation _worlddirection (.z (CallFunction|GetCenterLocation))))
    (Variables|Default|SetTargetLookXY _targetpoint)))

(fn ApplyRotation
  (if (> (Math|Float|Absolute(Float) (Variables|Default|GetAimDeltaYaw)) 1e+02)
    (if (Variables|Default|GetIsTurningLeft)
      (Class|Actor|AddActorWorldRotation "0.000000,-8.000000,0.000000")
      (elif (Variables|Default|GetIsTurningRight)
        (Class|Actor|AddActorWorldRotation "0.000000,8.000000,0.000000")))
    (elif (Variables|Default|GetIsTurningLeft)
      (Class|Actor|AddActorWorldRotation "0.000000,-4.000000,0.000000")
      (elif (Variables|Default|GetIsTurningRight)
        (Class|Actor|AddActorWorldRotation "0.000000,4.000000,0.000000")))))

(fn AdjustAimWeapon
  (bind _currentweapon (Variables|Default|GetCurrentWeapon))
  (bind _returnvalue (Transformation|GetActorLocation _currentweapon))
  (if (Variables|Default|GetIsAiming)
    (Transformation|SetActorRotation (Variables|Default|GetCurrentWeapon) (Math|Rotator|MakeRotator 0.0 0.0 (+ (.yaw (Math|Rotator|MakeRotfromX (Math|Vector|Normalize (- (Variables|Default|GetTargetLookXY) (Math|Vector|MakeVector (.x _returnvalue) (.y _returnvalue) 0.0))))) -9e+01)))))

(fn GetTargetLocAccordingtoZ
  (params (Origin :type Vector) (Direction :type Vector) (TargetZ :type Float%20%28double-precision%29))
  (return (+ (Math|Vector|MakeVector (.x Origin) (.y Origin) (.z Origin)) (* (/ (- TargetZ (.z Origin)) (.z Direction)) (Math|Vector|MakeVector (.x Direction) (.y Direction) (.z Direction))))))

(fn CanDoActions
  (params (NegateOutput :type Boolean))
  (bind _charactermovement (Variables|Character|GetCharacterMovement))
  (bind _isdodging (Variables|Default|GetIsDodging))
  (bind _isinteracting (Variables|Default|GetIsInteracting))
  (bind _returnvalue (AI|Components|NavMovement|IsFalling _charactermovement))
  (bind _returnvalue_2 (Math|Boolean|ORBoolean _returnvalue _isdodging _isinteracting))
  (if NegateOutput
    (return _returnvalue_2)
    (else
      (return (not _returnvalue_2)))))

(fn GetCenterLocation
  (bind _returnvalue (Transformation|GetActorLocation))
  (return (Math|Vector|MakeVector (.x _returnvalue) (.y _returnvalue) (+ (.z _returnvalue) (Variables|Default|GetLocalZ)))))

(fn InitArena
  (bind _healthcomponent (Variables|Default|GetHealthComponent))
  (bind _playerctrl (Variables|Default|GetPlayerCtrl))
  (bind _returnvalue (PlayerController|LocalPlayerSubsystems|GetEnhancedInputLocalPlayerSubsystem _playerctrl))
  (Utilities|FlowControl|Sequence
    (:then_0
      (Class|EnhancedInputSubsystemInterface|ClearAllMappings _returnvalue)
      (Input|AddMappingContext _returnvalue "/Game/_Main/Input/IMC_Game.IMC_Game" 0 "(bIgnoreAllPressedKeysUntilRelease=True,bForceImmediately=False,bNotifyUserSettings=False)"))
    (:then_1
      (CallFunction|SwitchtoCamera)
      (CallFunction|SetRunSpeed)
      (Variables|Default|SetIsInteracting false)
      (Variables|Default|SetIsInLab false)
      (Variables|Default|SetIsDead false))
    (:then_2
      (bind _equippeditems (Default|GetEquippedItems (Variables|Default|GetGM_Game)))
      (bind _result (Utilities|Set|ToArray _equippeditems))
      (bind _output_get (Variables|Default|SetItems _result))
      (CallFunction|SpawnWeapon (Utilities|Array|Get(acopy) _output_get))
      (bind (_dataasset _saveddata) (Default|GetSkillData (Variables|/Game/_Main/GM_Game.GM_Game_C|GetSaveGame (Variables|Default|GetGM_Game)) "/Game/_Main/Data/Skills/Skill_HP.Skill_HP"))
      (if (> (.CurrentLevel (Utilities|Struct|BreakSkillSavedData _saveddata)) 0)
        (bind _skillleveldata (Default|GetDataforLevel _dataasset (.CurrentLevel (Utilities|Struct|BreakSkillSavedData _saveddata))))
        (Variables|/Game/_Main/Components/HealthComponent.HealthComponent_C|SetHealthPoints _healthcomponent (+ (.upgrade _skillleveldata) (Variables|/Game/_Main/Components/HealthComponent.HealthComponent_C|GetHealthPoints _healthcomponent)))))))

(fn InitLab
  (bind _playerctrl (Variables|Default|GetPlayerCtrl))
  (bind _returnvalue (PlayerController|LocalPlayerSubsystems|GetEnhancedInputLocalPlayerSubsystem _playerctrl))
  (Utilities|FlowControl|Sequence
    (:then_0
      (Variables|Default|SetIsInteracting false)
      (Variables|Default|SetIsInLab true)
      (CallFunction|SetWalkSpeed))
    (:then_1
      (Class|EnhancedInputSubsystemInterface|ClearAllMappings _returnvalue)
      (Input|AddMappingContext _returnvalue "/Game/_Main/Input/IMC_Lab.IMC_Lab" 0 "(bIgnoreAllPressedKeysUntilRelease=True,bForceImmediately=False,bNotifyUserSettings=False)"))
    (:then_2
      (Actor|DestroyActor (Variables|Default|GetCurrentWeapon)))))

(fn TickArena
  (params (DeltaTime :type Float%20%28double-precision%29))
  (Utilities|FlowControl|Sequence
    (:then_0
      (if (Variables|Default|GetIsDodging)
        (CallFunction|TickRoll DeltaTime)
        (elif (Variables|Default|GetIsAiming)
          (CallFunction|TickLookat))))
    (:then_1
      (Default|UpdateHUD (Variables|Default|GetCurrentWeapon)))))

(fn SwitchtoCamera
  (params (Camera :type BP%20Camera%20Object%20Reference))
  (bind _asbp_camera (Utilities|Casting|CastToBP_Camera (Utilities|SelectObject Camera (Variables|/Script/Engine.ChildActorComponent|GetChildActor (Variables|Default|GetBP_Camera)) (Utilities|IsValid Camera))))
  (bind _output_get (Variables|Default|SetCurrentCam _asbp_camera))
  (bind _asplayer_controller (Utilities|Casting|CastToPlayerController (Pawn|GetController)))
  (Game|Player|SetViewTargetwithBlend _asplayer_controller _output_get 0.0 "VTBlend_Linear" 0.0 false))

(fn ResetInteraction
  (Variables|Default|SetCanInteract true)
  (Variables|Default|SetIsInteracting false))