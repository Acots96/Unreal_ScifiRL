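; BP_LabLead is an NPC that shows welcome dialogue through GM_Game when the player interacts with it.
; Capsule overlaps register its InteractComponent on BP_Character and toggle the interact widget and HUD prompt.
; On interact, it also limits its SceneCaptureComponent2D to its own components.
; Tick spins the widget, bobs a drone mesh on a sine wave and eases the character mesh's rotation toward the nearby player.
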(event `OnInteract`
  (`/Game/_Main/GM_Game.ShowDialogueHUD` (`self.GM_Game`) (`self.WelcomeText`))
  (`SceneCaptureComponent.ShowOnlyActorComponents` (`self.SceneCaptureComponent2D`) self false))

(event `OnBeginEnd`
  (params (OverlappedComponent :type "PrimitiveComponent Object Reference") (OtherActor :type "Actor Object Reference") (OtherComp :type "PrimitiveComponent Object Reference") (OtherBodyIndex :type Integer))
  (if (`self.ActorHasTag` OtherActor "Player")
    (bind _asbp_character (cast `/Game/_Main/Characters/Main/BP_Character` OtherActor))
    (set `/Game/_Main/Characters/Main/BP_Character.CurrentInteractComp` null _asbp_character)
    (set `self.CharacterNear` null)
    (`SceneComponent.SetHiddenInGame` (`self.CanInteract_Widget`) true false)
    (`/Game/_Main/GM_Game.CleanMessageHUD` (`self.GM_Game`))))

(event `self.ReceiveBeginPlay`
  (bind _capsule (`self.Capsule`))
  (add `PrimitiveComponent.OnComponentBeginOverlap` _capsule (delegate `OnBeginOverlap`))
  (add `PrimitiveComponent.OnComponentEndOverlap` _capsule (delegate `OnBeginEnd`))
  (bind _asgm_game (cast `/Game/_Main/GM_Game` (`GameplayStatics.GetGameMode`)))
  (set `self.GM_Game` _asgm_game)
  (add `/Game/_Main/Components/InteractComponent.OnInteract` (`self.InteractComponent`) (delegate `OnInteract`)))

(event `OnBeginOverlap`
  (params (OverlappedComponent :type "PrimitiveComponent Object Reference") (OtherActor :type "Actor Object Reference") (OtherComp :type "PrimitiveComponent Object Reference") (OtherBodyIndex :type Integer) (bFromSweep :type Boolean) (SweepResult :type "HitResult Structure (by ref)"))
  (if (`self.ActorHasTag` OtherActor "Player")
    (bind _asbp_character (cast `/Game/_Main/Characters/Main/BP_Character` OtherActor))
    (set `/Game/_Main/Characters/Main/BP_Character.CurrentInteractComp` (`self.InteractComponent`) _asbp_character)
    (set `self.CharacterNear` _asbp_character)
    (`SceneComponent.SetHiddenInGame` (`self.CanInteract_Widget`) false false)
    (`/Game/_Main/GM_Game.ShowMessageHUD` (`self.GM_Game`) "Press E to interact" 0.0)))

(event `self.ReceiveTick`
  (params (DeltaSeconds :type "Float (single-precision)"))
  (`self.RotateWidgetBottom` DeltaSeconds)
  (`self.FloatingEffect` DeltaSeconds)
  (`self.ComputeLookAt`))

(fn `ComputeLookAt`
  (locals (Local_TargetRot :type "Rotator Structure"))
  (bind _charmesh (`self.CharMesh`))
  (bind (_returnvalue_roll _returnvalue_pitch _returnvalue_yaw) (`KismetMathLibrary.BreakRotator` (`KismetMathLibrary.MakeRotFromX` (`KismetMathLibrary.Vector_Normal2D` (- (`self.K2_GetActorLocation` (`self.CharacterNear`)) (`self.K2_GetActorLocation`))))))
  (`|ExecutionSequence`
    (:`then_0`
      (`/Engine/EditorBlueprintResources/StandardMacros.IsValid` (`self.CharacterNear`)
        (:`Is Valid`
          (set `local.Local_TargetRot` (`KismetMathLibrary.MakeRotator` _returnvalue_roll _returnvalue_pitch (+ _returnvalue_yaw -90.0))))
        (:`Is Not Valid`
          (set `local.Local_TargetRot` (struct)))))
    (:`then_1`
      (`SceneComponent.K2_SetWorldRotation` _charmesh (`KismetMathLibrary.RLerp` (`SceneComponent.K2_GetComponentRotation` _charmesh) (`local.Local_TargetRot`) 0.05 true) false false))))

(fn `FloatingEffect`
  (params (DeltaTime :type "Float (double-precision)"))
  (bind _output_get (set `self.ZEffect` (+ (* DeltaTime 50.0) (`self.ZEffect`))))
  (`SceneComponent.K2_SetRelativeLocation` (`self.DroneMesh`) (`KismetMathLibrary.MakeVector` 0.0 0.0 (* (`KismetMathLibrary.DegSin` _output_get) 2.0)) false false))

(fn `RotateWidgetBottom`
  (params (DeltaTime :type "Float (double-precision)"))
  (`SceneComponent.K2_AddRelativeRotation` (`self.CanInteract_Widget`) (`KismetMathLibrary.MakeRotator` 0.0 0.0 (* DeltaTime 100.0)) false false))

(fn `UserConstructionScript`)