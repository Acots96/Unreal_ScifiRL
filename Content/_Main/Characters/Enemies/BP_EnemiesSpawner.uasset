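; BP_EnemiesSpawner is an enemy spawner that places enemies at random points inside its BoxArea.
; SpawnEnemiesFromData spawns each data entry's enemy class, passes that entry in as WaveData and returns the spawned actors.
; Random points vary in X and Y within the box bounds and keep the center height.
; BeginPlay is empty and the Amount-based loop is unwired, so spawning happens only when its functions are called.
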(event `self.ReceiveBeginPlay`)

(fn `GetAllEnemies`
  (returns (Enemies :type "Array of /Game/_Main/Characters/Enemies/BP_Enemy Object Reference"))
  (return (`self.Enemies`)))

(fn `GetRandomLocationInArea`
  (returns (Location :type "Vector Structure"))
  (bind (_origin _boxextent) (`KismetSystemLibrary.GetComponentBounds` (`self.BoxArea`)))
  (return (+ _origin (`KismetMathLibrary.MakeVector` (* (.x _boxextent) (- (* (`KismetMathLibrary.RandomFloat`) 2.0) 1.0)) (* (.y _boxextent) (- (* (`KismetMathLibrary.RandomFloat`) 2.0) 1.0))))))

(fn `SpawnEnemiesFromData`
  (params (EnemiesData :type "Array of /Game/_Main/Characters/Enemies/EnemyWaveData Object Reference"))
  (returns (Enemies :type "Array of /Game/_Main/Characters/Enemies/BP_Enemy Object Reference"))
  (locals (Local_Enemies :type "Array of /Game/_Main/Characters/Enemies/BP_Enemy Object Reference"))
  (for _array_element EnemiesData
    (bind _enemy (`self.SpawnEnemy` _array_element))
    (`KismetArrayLibrary.Array_Add` (`local.Local_Enemies`) _enemy))
  (return (`local.Local_Enemies`)))

(fn `SpawnEnemy`
  (params (EnemyData :type "/Game/_Main/Characters/Enemies/EnemyWaveData Object Reference"))
  (returns (Enemy :type "/Game/_Main/Characters/Enemies/BP_Enemy Object Reference"))
  (bind _returnvalue (`|SpawnActorFromClass` (`/Game/_Main/Characters/Enemies/EnemyWaveData.BP_Enemy` EnemyData) (`KismetMathLibrary.MakeTransform` (`self.GetRandomLocationInArea`)) "Undefined" "MultiplyWithRoot" null null EnemyData null))
  (return _returnvalue))

(fn `UserConstructionScript`)