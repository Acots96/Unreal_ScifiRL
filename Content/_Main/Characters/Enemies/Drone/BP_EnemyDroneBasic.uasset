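; Basic flying drone enemy that keeps a mid-range distance from the player and fires laser projectiles.
; A 0.2s loop picks its destination, adding repulsion from other wave enemies.
; Tick eases speed by distance, moves without sweep, yaws toward the target, and fires when slow, level and aimed.
; A poseable mesh gets procedural bob, tilt and booster rotation; health events update the bar, and death awards score and spawns an explosion.
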(event `self.ReceiveBeginPlay`
  (bind _healthcomponent (`self.HealthComponent`))
  (`|ExecutionSequence`
    (:`then_0`
      (bind _returnvalue (`GameplayStatics.GetActorOfClass` "/Game/_Main/Characters/Main/BP_Character.BP_Character_C"))
      (set `self.Target` _returnvalue)
      (`self.ComputeDesiredLocation` :!label _label)
      (`KismetSystemLibrary.Delay` 0.2)
      (goto _label))
    (:`then_1`
      (bind _aswbp_health (cast `/Game/_Main/UI/WBP_Health` (`WidgetComponent.GetWidget` (`self.HealthBarWidget`))))
      (bind _output_get (set `self.HealthWidget` _aswbp_health))
      (`/Game/_Main/UI/WBP_Health.SetLifeBarFraction` _output_get 1.0)
      (add `/Game/_Main/Components/HealthComponent.OnDied` _healthcomponent (delegate `OnDiedEvent`))
      (add `/Game/_Main/Components/HealthComponent.OnDamaged` _healthcomponent (delegate `OnDamagedEvent`)))
    (:`then_2`
      (`self.InitializeThrustersVFX`))))

(event `OnDiedEvent`
  (params (Damage :type "Float (double-precision)") (Attacker :type "Actor Object Reference"))
  (`self.Died`))

(event `OnDamagedEvent`
  (params (Damage :type "Float (double-precision)") (Attacker :type "Actor Object Reference"))
  (`self.Damaged`))

(event `self.ReceiveTick`
  (params (DeltaSeconds :type "Float (single-precision)"))
  (if (not (`/Game/_Main/Components/HealthComponent.IsDead` (`self.HealthComponent`)))
    (`|ExecutionSequence`
      (:`then_0`
        (`self.ComputeSpeed`)
        (`self.MoveDrone` DeltaSeconds))
      (:`then_1`
        (`self.TickLaser` DeltaSeconds)))))

(fn `ComputeDesiredLocation`
  (bind (_returnvalue_x _returnvalue_y) (`KismetMathLibrary.BreakVector` (`self.K2_GetActorLocation`)))
  (bind (_returnvalue_x_2 _returnvalue_y_2) (`KismetMathLibrary.BreakVector` (`self.K2_GetActorLocation` (`self.Target`))))
  (bind (_loc_x _loc_y _loc_z) (`KismetMathLibrary.BreakVector` (`/Game/_Main/Characters/Main/BP_Character.GetCenterLocation` (`self.Target`))))
  (bind _repulsionvector (`self.ComputeRepulsionVectors`))
  (bind (_returnvalue_x_3 _returnvalue_y_3) (`KismetMathLibrary.BreakVector` (+ _repulsionvector (* (`KismetMathLibrary.Normal` (- (`KismetMathLibrary.MakeVector` _returnvalue_x _returnvalue_y) (`KismetMathLibrary.MakeVector` _returnvalue_x_2 _returnvalue_y_2))) (* (+ (`self.MaxDistToTarget`) (`self.MinDistToTarget`)) 0.5)) (`KismetMathLibrary.MakeVector` _loc_x _loc_y))))
  (set `self.DesiredLocation` (`KismetMathLibrary.MakeVector` _returnvalue_x_3 _returnvalue_y_3 _loc_z)))

(fn `ComputeDirection`
  (returns (Direction :type "Vector Structure"))
  (return (`KismetMathLibrary.SelectVector` (`self.GetDirectionToDesiredLocation`) (`self.GetActorForwardVector`) (> (`self.DesiredSpeed`) 0.1))))

(fn `ComputeMovementEffect`
  (params (DeltaTime :type "Float (double-precision)"))
  (bind _poseablemesh (`self.PoseableMesh`))
  (bind _poseablemesh_2 (`self.PoseableMesh`))
  (bind _currentspeed (`self.CurrentSpeed`))
  (bind _poseablemesh_3 (`self.PoseableMesh`))
  (bind _poseablemesh_4 (`self.PoseableMesh`))
  (bind (_returnvalue_x _returnvalue_y) (`KismetMathLibrary.BreakVector` (`KismetMathLibrary.InverseTransformDirection` (`self.GetTransform`) (`self.ComputeDirection`))))
  (bind _returnvalue_x_2 (`KismetMathLibrary.BreakVector` (`KismetMathLibrary.InverseTransformDirection` (`self.GetTransform`) (`self.ComputeDirection`))))
  (bind _returnvalue_x_3 (`KismetMathLibrary.BreakVector` (`KismetMathLibrary.InverseTransformDirection` (`self.GetTransform`) (`self.ComputeDirection`))))
  (bind (_relativelocation_x _relativelocation_y _relativelocation_z) (`KismetMathLibrary.BreakVector` (`SceneComponent.RelativeLocation` _poseablemesh)))
  (bind _relativerotation (`SceneComponent.RelativeRotation` _poseablemesh_2))
  (`/Engine/EditorBlueprintResources/StandardMacros.IsValid` (`self.PoseableMesh`)
    (:`Is Valid`
      (`|ExecutionSequence`
        (:`then_0`
          (if (<= (`self.CurrentSpeed`) (`self.FastSpeed`))
            (bind _output_get (set `self.ZEffectDelta` (+ (`self.ZEffectDelta`) (* DeltaTime (`self.FloatEffectSpeed`)))))
            (`SceneComponent.K2_SetRelativeLocation` _poseablemesh (`KismetMathLibrary.MakeVector` 0.0 0.0 (+ _relativelocation_z (* (`KismetMathLibrary.Sin` _output_get) (`self.FloatEffectAmplitude`)))) false false)))
        (:`then_1`
          (`SceneComponent.K2_SetRelativeRotation` _poseablemesh_2 (`KismetMathLibrary.RLerp` _relativerotation (`KismetMathLibrary.MakeRotator` (* _returnvalue_y (`self.FloatEffectRotRollMult`) _currentspeed) (* _returnvalue_x (`self.FloatEffectRotPitchMult`) _currentspeed)) (`self.FloatEffectRotLerpSpeed`) true) false false)
          (set `self.CanShootLaser` (< (`KismetMathLibrary.Abs` (.pitch _relativerotation)) 10.0))
          (`|ExecutionSequence`
            (:`then_0`
              (bind _returnvalue (`PoseableMeshComponent.GetBoneRotationByName` _poseablemesh_3 "SM_Prop_Drone_03_l_Booster_01" "ComponentSpace"))
              (bind (_returnvalue_roll _returnvalue_pitch) (`KismetMathLibrary.BreakRotator` (`KismetMathLibrary.RLerp` (`KismetMathLibrary.MakeRotator` 0.0 (.pitch _returnvalue)) (`KismetMathLibrary.MakeRotator` 0.0 (+ (* _returnvalue_x_2 (`self.BoosterEffectPitchSpeed`) (`self.CurrentSpeed`)) 90.0)) (`self.BoosterEffectLerpSpeed`) true)))
              (`PoseableMeshComponent.SetBoneRotationByName` _poseablemesh_3 "SM_Prop_Drone_03_l_Booster_01" (`KismetMathLibrary.MakeRotator` 0.0 _returnvalue_pitch) "ComponentSpace"))
            (:`then_1`
              (bind _returnvalue_2 (`PoseableMeshComponent.GetBoneRotationByName` _poseablemesh_4 "SM_Prop_Drone_03_r_Booster_01" "ComponentSpace"))
              (bind (_returnvalue_roll_2 _returnvalue_pitch_2) (`KismetMathLibrary.BreakRotator` (`KismetMathLibrary.RLerp` (`KismetMathLibrary.MakeRotator` 0.0 (.pitch _returnvalue_2)) (`KismetMathLibrary.MakeRotator` 0.0 (+ (* _returnvalue_x_3 (`self.BoosterEffectPitchSpeed`) (`self.CurrentSpeed`)) 90.0)) (`self.BoosterEffectLerpSpeed`) true)))
              (`PoseableMeshComponent.SetBoneRotationByName` _poseablemesh_4 "SM_Prop_Drone_03_r_Booster_01" (`KismetMathLibrary.MakeRotator` 0.0 _returnvalue_pitch_2) "ComponentSpace"))))))))

(fn `ComputeRepulsionVectors`
  (returns (RepulsionVector :type "Vector Structure"))
  (locals (Local_Vector :type "Vector Structure") (Local_MinDist :type "Float (double-precision)" :default 200.0) (Local_CheckDist :type "Float (double-precision)" :default 1000.0))
  (bind _wavesmanager (`self.WavesManager`))
  (`/Engine/EditorBlueprintResources/StandardMacros.IsValid` _wavesmanager
    (:`Is Valid`
      (for _array_element (`/Game/_Main/BP_WavesManager.GetAllEnemies` _wavesmanager)
        (`/Engine/EditorBlueprintResources/StandardMacros.IsValid` _array_element
          (:`Is Valid`
            (if (!= _array_element self)
              (bind _returnvalue (- (`self.K2_GetActorLocation`) (`self.K2_GetActorLocation` _array_element)))
              (bind _returnvalue_2 (`KismetMathLibrary.VSizeXY` _returnvalue))
              (if (<= _returnvalue_2 (`local.Local_CheckDist`))
                (set `local.Local_Vector` (+ (`local.Local_Vector`) (* (`KismetMathLibrary.FClamp` (/ (`local.Local_MinDist`) _returnvalue_2)) (`local.Local_MinDist`) (`KismetMathLibrary.Normal` _returnvalue)))))))))
      (return (`local.Local_Vector`)))))

(fn `ComputeRotationWhenShooting`
  (params (DeltaTime :type "Float (double-precision)"))
  (locals (Local_Angle :type "Float (double-precision)" :default 0.0))
  (bind _output_get (set `local.Local_Angle` (`KismetMathLibrary.DegAcos` (`KismetMathLibrary.Dot_VectorVector` (`self.GetDirectionToTarget`) (`self.GetActorForwardVector`)))))
  (if (> _output_get 10.0)
    _
    (else
      _))
  (`self.K2_AddActorWorldRotation` (`KismetMathLibrary.MakeRotator` 0.0 0.0 (* (`KismetMathLibrary.SelectFloat` 1.0 -1.0 (< (`KismetMathLibrary.Dot_VectorVector` (`KismetMathLibrary.Cross_VectorVector` (`self.GetDirectionToTarget`) (`self.GetActorForwardVector`)) (`self.GetActorUpVector`)) 0.0)) DeltaTime (`self.RotationSpeedWhenShooting`)))))

(fn `ComputeSpeed`
  (locals (Local_Dist :type "Float (double-precision)" :default 0.0))
  (bind (_returnvalue_x _returnvalue_y) (`KismetMathLibrary.BreakVector` (`self.K2_GetActorLocation`)))
  (bind (_desiredlocation_x _desiredlocation_y) (`KismetMathLibrary.BreakVector` (`self.DesiredLocation`)))
  (bind _output_get (set `local.Local_Dist` (`KismetMathLibrary.Distance2D` (`KismetMathLibrary.MakeVector2D` _desiredlocation_x _desiredlocation_y) (`KismetMathLibrary.MakeVector2D` _returnvalue_x _returnvalue_y))))
  (if (> _output_get (`self.MaxDistToTarget`))
    (set `self.DesiredSpeed` (`self.FastSpeed`))
    (elif (> (`KismetMathLibrary.Distance2D` (`KismetMathLibrary.MakeVector2D` _returnvalue_x _returnvalue_y) (`KismetMathLibrary.MakeVector2D` _desiredlocation_x _desiredlocation_y)) (`self.StopDistToTarget`))
      (set `self.DesiredSpeed` (`self.StillSpeed`))
      (else
        (set `self.DesiredSpeed` 0.0)))))

(fn `Damaged`
  (`/Game/_Main/UI/WBP_Health.SetLifeBarFraction` (`self.HealthWidget`) (`/Game/_Main/Components/HealthComponent.GetFraction` (`self.HealthComponent`))))

(fn `Died`
  (`|ExecutionSequence`
    (:`then_0`
      (`self.SetActorTickEnabled` false)
      (bind _asgm_game (cast `/Game/_Main/GM_Game` (`GameplayStatics.GetGameMode`)))
      (`/Game/_Main/GM_Game.SpawnScore` _asgm_game (`/Game/_Main/Characters/Enemies/EnemyWaveData.Score` (`self.WaveData`)) (`self.K2_GetActorLocation`)))
    (:`then_1`
      (`|SpawnActorFromClass` (`self.BP_DieExplosion`) (`KismetMathLibrary.MakeTransform` (`self.K2_GetActorLocation`)) "Undefined" "MultiplyWithRoot" null null))
    (:`then_2`
      (`self.K2_DestroyActor`))))

(fn `GetDirectionToDesiredLocation`
  (returns (ReturnValue :type "Vector Structure"))
  (return (`KismetMathLibrary.Normal` (- (`self.DesiredLocation`) (`self.K2_GetActorLocation`)))))

(fn `GetDirectionToTarget`
  (returns (Direction :type "Vector Structure"))
  (return (`KismetMathLibrary.Normal` (- (`/Game/_Main/Characters/Main/BP_Character.GetCenterLocation` (`self.Target`)) (`self.K2_GetActorLocation`)))))

(fn `GetDistanceToTarget`
  (returns (Distance :type "Float (double-precision)"))
  (return (`KismetMathLibrary.VSizeXY` (- (`/Game/_Main/Characters/Main/BP_Character.GetCenterLocation` (`self.Target`)) (`self.K2_GetActorLocation`)))))

(fn `InitializeThrustersVFX`
  (`SceneComponent.K2_AttachToComponent` (`self.Niagara_ThrusterL`) (`self.PoseableMesh`) "Socket_BoosterL" "SnapToTarget" "SnapToTarget" "KeepWorld" true)
  (`SceneComponent.K2_AttachToComponent` (`self.Niagara_ThrusterR`) (`self.PoseableMesh`) "Socket_BoosterR" "SnapToTarget" "SnapToTarget" "KeepWorld" true))

(fn `MoveDrone`
  (params (DeltaTime :type "Float (double-precision)"))
  (`self.TickSpeed` DeltaTime)
  (`|ExecutionSequence`
    (:`then_0`
      (`self.K2_AddActorWorldOffset` (* DeltaTime (`self.CurrentSpeed`) (`self.ComputeDirection`))))
    (:`then_1`
      (`self.ComputeRotationWhenShooting` DeltaTime)
      (`self.ComputeMovementEffect` DeltaTime))))

(fn `ShootLaser`
  (bind (_returnvalue_location _returnvalue_rotation) (`KismetMathLibrary.BreakTransform` (`SceneComponent.K2_GetComponentToWorld` (`self.ShooterLaser`))))
  (`|ExecutionSequence`
    (:`then_0`
      (`|SpawnActorFromClass` (`self.BP_Projectile`) (`KismetMathLibrary.MakeTransform` _returnvalue_location _returnvalue_rotation) "Undefined" "OverrideRootScale" self (`self.TargetTags`) (`self.Damage`) null)
      (`ActorComponent.Activate` (`self.Niagara_LaserMuzzle`) true))))

(fn `TickLaser`
  (params (DeltaTime :type "Float (double-precision)"))
  (if (`self.CanShootLaser`)
    (bind _output_get (set `self.LaserDelayDelta` (- (`self.LaserDelayDelta`) DeltaTime)))
    (if (and (<= _output_get 0.0) (< (`self.CurrentSpeed`) (`self.FastSpeed`)) (>= (`KismetMathLibrary.Dot_VectorVector` (`self.GetDirectionToTarget`) (`self.GetActorForwardVector`)) 0.99))
      (`self.ShootLaser`)
      (set `self.LaserDelayDelta` (`self.LaserDelay`)))))

(fn `TickSpeed`
  (params (DeltaTime :type "Float (double-precision)"))
  (set `self.CurrentSpeed` (+ (* (`KismetMathLibrary.SignOfFloat` (- (`self.DesiredSpeed`) (`self.CurrentSpeed`))) (`self.Acceleration`) DeltaTime) (`self.CurrentSpeed`))))

(fn `UserConstructionScript`)