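; Mid-tier enemy drone that adds homing-style missile volleys to the movement and laser attack of its parent class.
; While alive it moves and ticks both weapons, launching a volley on a randomized cooldown when below its fast speed and resetting the laser delay.
; A looping timer spawns missiles from the shooter component, passing target, tags and damage, until the volley count runs out.
; The missile muzzle Niagara effect is disconnected.
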(event `self.ReceiveBeginPlay`
  (bind _missilesdelay (`self.MissilesDelay`))
  (`parent.ReceiveBeginPlay`)
  (set `self.MissilesDelayDelta` (`KismetMathLibrary.RandomFloatInRange` (+ _missilesdelay -1.0) (+ _missilesdelay 1.0))))

(event `self.ReceiveTick`
  (params (DeltaSeconds :type "Float (single-precision)"))
  (if (not (`/Game/_Main/Components/HealthComponent.IsDead` (`self.HealthComponent`)))
    (`|ExecutionSequence`
      (:`then_0`
        (`self.ComputeSpeed`)
        (`self.MoveDrone` DeltaSeconds))
      (:`then_1`
        (`self.TickLaser` DeltaSeconds)
        (`self.TickMissiles` DeltaSeconds)))))

(event `ShootMissiles`
  (set `self.MissilesToSpawnDelta` (`self.MissilesToSpawn`))
  (`KismetSystemLibrary.K2_SetTimer` null "SpawnMissile" (`self.BewteenMissilesDelay`) true))

(fn `SpawnMissile`
  (bind (_returnvalue_location _returnvalue_rotation) (`KismetMathLibrary.BreakTransform` (`SceneComponent.K2_GetComponentToWorld` (`self.ShooterMissiles`))))
  (`|SpawnActorFromClass` (`self.BP_Missile`) (`KismetMathLibrary.MakeTransform` _returnvalue_location _returnvalue_rotation) "Undefined" "OverrideRootScale" self (`self.Target`) (`self.TargetTags`) (`self.Damage`) null)
  (bind _result (`/Engine/EditorBlueprintResources/StandardMacros.DecrementInt` (`self.MissilesToSpawnDelta`))
    (:`  `
      (if (<= _result 0)
        (`KismetSystemLibrary.K2_ClearTimer` null "SpawnMissile")))))

(fn `TickMissiles`
  (params (DeltaTime :type "Float (double-precision)"))
  (bind _missilesdelay (`self.MissilesDelay`))
  (bind _output_get (set `self.MissilesDelayDelta` (- (`self.MissilesDelayDelta`) DeltaTime)))
  (if (and (<= _output_get 0.0) (< (`self.CurrentSpeed`) (`self.FastSpeed`)) true)
    (set `self.LaserDelayDelta` 2.0)
    (`self.ShootMissiles`)
    (set `self.MissilesDelayDelta` (`KismetMathLibrary.RandomFloatInRange` (+ _missilesdelay -1.0) (+ _missilesdelay 1.0)))))

(fn `UserConstructionScript`
  (`parent.UserConstructionScript`))