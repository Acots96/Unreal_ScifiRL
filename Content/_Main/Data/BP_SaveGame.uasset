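; Save game Blueprint that stores player score, level progression, and saved skill and item levels.
; AddScore accumulates score, levels up on reaching the target and carries the excess, with each next target generated by a Fibonacci-style sequence.
; GetSkillData and GetItemData synchronously load data assets by path and return them with their saved entries, adding level-zero entries when missing.
; InitSlot resets score, target and level to starting values.
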(fn `AddScore`
  (params (Score :type Integer))
  (returns (ReachedNextLevel :type Boolean))
  (bind _currenttargetscore (`self.CurrentTargetScore`))
  (set `self.TotalScore` (+ Score (`self.TotalScore`)))
  (bind _output_get (set `self.CurrentScore` (+ (`self.CurrentScore`) Score)))
  (if (>= _output_get _currenttargetscore)
    (`/Engine/EditorBlueprintResources/StandardMacros.IncrementInt` (`self.CurrentLevel`)
      (:`  `
        (set `self.CurrentScore` (- (`self.CurrentScore`) _currenttargetscore))
        (bind _targetscore (`self.GetNextTargetScore`))
        (set `self.CurrentTargetScore` _targetscore)
        (return true)))
    (else
      (return false))))

(fn `GetItemData`
  (params (ItemDataPath :type "/Game/_Main/Data/Items/ItemDataAsset Soft Object Reference"))
  (returns (DataAsset :type "/Game/_Main/Data/Items/ItemDataAsset Object Reference") (SavedData :type "/Game/_Main/Data/Items/ItemSavedData Structure"))
  (bind _itemssaved (`self.ItemsSaved`))
  (bind (_value _returnvalue) (`BlueprintMapLibrary.Map_Find` _itemssaved ItemDataPath))
  (bind _returnvalue_2 (`KismetSystemLibrary.LoadAsset_Blocking` ItemDataPath))
  (bind _asitem_data_asset (cast `/Game/_Main/Data/Items/ItemDataAsset` _returnvalue_2))
  (if _returnvalue
    (return _asitem_data_asset _value)
    (else
      (`BlueprintMapLibrary.Map_Add` _itemssaved ItemDataPath (make `/Game/_Main/Data/Items/ItemSavedData` ItemDataPath))
      (return _asitem_data_asset (make `/Game/_Main/Data/Items/ItemSavedData` ItemDataPath)))))

(fn `GetNextTargetScore`
  (returns (TargetScore :type Integer))
  (locals (Local_N :type Integer :default 3) (`Local_N+1` :type Integer :default 5) (Local_Aux :type Integer))
  (while (>= (`self.CurrentTargetScore`) (`local.Local_N+1`))
    (set `local.Local_Aux` (+ (`local.Local_N`) (`local.Local_N+1`)))
    (set `local.Local_N` (`local.Local_N+1`))
    (set `local.Local_N+1` (`local.Local_Aux`)))
  (return (`local.Local_N+1`)))

(fn `GetSkillData`
  (params (SkillDataPath :type "/Game/_Main/Data/Skills/SkillDataAsset Soft Object Reference"))
  (returns (DataAsset :type "/Game/_Main/Data/Skills/SkillDataAsset Object Reference") (SavedData :type "/Game/_Main/Data/Skills/SkillSavedData Structure"))
  (bind _skillssaved (`self.SkillsSaved`))
  (bind (_value _returnvalue) (`BlueprintMapLibrary.Map_Find` _skillssaved SkillDataPath))
  (bind _returnvalue_2 (`KismetSystemLibrary.LoadAsset_Blocking` SkillDataPath))
  (bind _asskill_data_asset (cast `/Game/_Main/Data/Skills/SkillDataAsset` _returnvalue_2))
  (if _returnvalue
    (return _asskill_data_asset _value)
    (else
      (`BlueprintMapLibrary.Map_Add` _skillssaved SkillDataPath (make `/Game/_Main/Data/Skills/SkillSavedData` SkillDataPath))
      (return _asskill_data_asset (make `/Game/_Main/Data/Skills/SkillSavedData` SkillDataPath)))))

(fn `InitSlot`
  (`|ExecutionSequence`
    (:`then_0`
      (set `self.TotalScore` 0))
    (:`then_1`
      (set `self.CurrentScore` 0))
    (:`then_2`
      (set `self.CurrentTargetScore` 13))
    (:`then_3`
      (set `self.CurrentLevel` 1))))