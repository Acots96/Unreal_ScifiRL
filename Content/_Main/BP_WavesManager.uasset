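; Wave manager that spawns escalating drone waves, starting the next wave when all current enemies are destroyed.
; BeginPlay finds the BP_EnemiesSpawner and builds a table of drone types with score costs, without starting a wave itself.
; InitNextWave raises the score budget, fills it with random affordable enemy picks and passes them to the spawner.
; Spawned enemies are tracked through OnDestroyed bindings and receive a reference to the manager.
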(event `self.ReceiveBeginPlay`
  (`|ExecutionSequence`
    (:`then_0`
      (bind _returnvalue (`GameplayStatics.GetActorOfClass` "/Game/_Main/Characters/Enemies/BP_EnemiesSpawner.BP_EnemiesSpawner_C"))
      (set `self.EnemiesSpawner` _returnvalue))
    (:`then_1`
      (`self.CreateEnemiesData`))))

(fn `CreateEnemiesData`
  (`|ExecutionSequence`
    (:`then_0`
      (`KismetArrayLibrary.Array_Clear` (`self.EnemiesData`)))
    (:`then_1`
      (bind _returnvalue (`|GenericCreateObject` "/Game/_Main/Characters/Enemies/EnemyWaveData.EnemyWaveData_C" "/Game/_Main/Characters/Enemies/Drone/BP_EnemyDroneBasic.BP_EnemyDroneBasic_C" 2))
      (`KismetArrayLibrary.Array_Add` (`self.EnemiesData`) _returnvalue))
    (:`then_2`
      (bind _returnvalue_2 (`|GenericCreateObject` "/Game/_Main/Characters/Enemies/EnemyWaveData.EnemyWaveData_C" "/Game/_Main/Characters/Enemies/Drone/BP_EnemyDroneMid.BP_EnemyDroneMid_C" 5))
      (`KismetArrayLibrary.Array_Add` (`self.EnemiesData`) _returnvalue_2))))

(fn `GenerateEnemiesCombination`
  (params (Points :type Integer))
  (returns (Enemies :type "Array of /Game/_Main/Characters/Enemies/EnemyWaveData Object Reference"))
  (locals (Local_Enemies :type "Array of /Game/_Main/Characters/Enemies/EnemyWaveData Object Reference") (Local_Points :type Integer) (Local_MaxCount :type Integer :default 10) (Local_Enemy :type "/Game/_Main/Characters/Enemies/EnemyWaveData Object Reference"))
  (bind _output_get (set `local.Local_Points` Points))
  (while (> _output_get 0)
    (bind _output_get_2 (set `local.Local_Enemy` (`KismetArrayLibrary.Array_Random` (`self.GetEnemiesUnderScore` (`local.Local_Points`)))))
    (`/Engine/EditorBlueprintResources/StandardMacros.IsValid` _output_get_2
      (:`Is Valid`
        (`KismetArrayLibrary.Array_Add` (`local.Local_Enemies`) _output_get_2)
        (set `local.Local_Points` (- (`local.Local_Points`) (`/Game/_Main/Characters/Enemies/EnemyWaveData.Score` _output_get_2))))
      (:`Is Not Valid`
        (set `local.Local_Points` 0))))
  (return (`local.Local_Enemies`)))

(fn `GetAllEnemies`
  (returns (Enemies :type "Array of /Game/_Main/Characters/Enemies/BP_Enemy Object Reference"))
  (return (`self.CurrentEnemies`)))

(fn `GetEnemiesUnderScore`
  (params (MaxScore :type Integer))
  (returns (Enemies :type "Array of /Game/_Main/Characters/Enemies/EnemyWaveData Object Reference"))
  (locals (Local_Enemies :type "Array of /Game/_Main/Characters/Enemies/EnemyWaveData Object Reference"))
  (for _array_element (`self.EnemiesData`)
    (if (<= (`/Game/_Main/Characters/Enemies/EnemyWaveData.Score` _array_element) MaxScore)
      (`KismetArrayLibrary.Array_Add` (`local.Local_Enemies`) _array_element)))
  (return (`local.Local_Enemies`)))

(fn `InitNextWave`
  (set `self.CurrentWaveScore` (+ (`self.CurrentWaveScore`) (`self.ScoreIncrement`)))
  (bind _enemies (`self.GenerateEnemiesCombination` (`self.CurrentWaveScore`)))
  (`self.SpawnEnemies` _enemies))

(fn `OnAllEnemiesDestroyed`
  (`self.InitNextWave`))

(fn `OnEnemyDestroyed`
  (params (DestroyedActor :type "Actor Object Reference"))
  (bind _currentenemies (`self.CurrentEnemies`))
  (bind _asbp_enemy (cast `/Game/_Main/Characters/Enemies/BP_Enemy` DestroyedActor))
  (`KismetArrayLibrary.Array_RemoveItem` _currentenemies _asbp_enemy)
  (if (`KismetArrayLibrary.Array_IsEmpty` _currentenemies)
    (`self.OnAllEnemiesDestroyed`)))

(fn `SpawnEnemies`
  (params (EnemiesData :type "Array of /Game/_Main/Characters/Enemies/EnemyWaveData Object Reference"))
  (bind _enemies (`/Game/_Main/Characters/Enemies/BP_EnemiesSpawner.SpawnEnemiesFromData` (`self.EnemiesSpawner`) EnemiesData))
  (for _array_element _enemies
    (`KismetArrayLibrary.Array_Add` (`self.CurrentEnemies`) _array_element)
    (set `/Game/_Main/Characters/Enemies/BP_Enemy.WavesManager` self _array_element)
    (add `self.OnDestroyed` _array_element (`|CreateDelegate` :!event `OnEnemyDestroyed`))))

(fn `UserConstructionScript`)